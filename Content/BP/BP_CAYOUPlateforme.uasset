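; Platform actor whose cube continuously grows and shrinks horizontally, starting from BeginPlay.
; Move uses a FlipFlop to alternate between playing a timeline toward a newly randomized X and Y scale and reversing it back to the base size.
; The timeline lerps the cube's relative scale with fixed height and calls Move again on Finished, forming an endless loop.
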(event `self.ReceiveBeginPlay`
  (`self.Move`))

(event `Move`
  (bind _returnvalue (`KismetMathLibrary.RandomFloatInRange` 6.0 20.0))
  (`/Engine/EditorBlueprintResources/StandardMacros.FlipFlop`
    (:`A`
      (set `self.x` _returnvalue)
      (set `self.y` _returnvalue)
      (bind (_direction _newtrack_0) (`Timeline|Timeline_0` :!label _label)
        (:`Update`
          (`SceneComponent.SetRelativeScale3D` (`self.Cube`) (`KismetMathLibrary.VLerp` (4.0 4.0 4.0) (`KismetMathLibrary.MakeVector` (`self.x`) (`self.y`) 4.0) _newtrack_0)))
        (:`Finished`
          (`self.Move`))))
    (:`B`
      (goto _label :!via `Reverse`))))

(fn `UserConstructionScript`)