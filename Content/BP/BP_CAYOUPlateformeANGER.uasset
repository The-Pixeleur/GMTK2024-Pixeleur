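; A platform that continually resizes and, when the first-person character enters its box, shakes and then drops away.
; A FlipFlop loop plays and reverses a timeline, stretching the cube's X and Y scale toward random sizes and back.
; Overlap resets a DoN that chains small random jitters through the Shake event.
; At count five the cube sinks far down, then rises back after a delay via a reversed timeline.
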(event `self.ReceiveBeginPlay`
  (`self.Move`))

(event `Move`
  (bind _returnvalue (`KismetMathLibrary.RandomFloatInRange` 6.0 20.0))
  (`/Engine/EditorBlueprintResources/StandardMacros.FlipFlop`
    (:`A`
      (set `self.x` _returnvalue)
      (set `self.y` _returnvalue)
      (bind (_direction _newtrack_0) (`Timeline|Timeline_0` :!label _label)
        (:`Update`
          (`SceneComponent.SetRelativeScale3D` (`self.Cube`) (`KismetMathLibrary.VLerp` (4.0 4.0 4.0) (`KismetMathLibrary.MakeVector` (`self.x`) (`self.y`) 4.0) _newtrack_0)))
        (:`Finished`
          (`self.Move`))))
    (:`B`
      (goto _label :!via `Reverse`))))

(event `self.Box.OnComponentBeginOverlap`
  (params (OverlappedComponent :type "PrimitiveComponent Object Reference") (OtherActor :type "Actor Object Reference") (OtherComp :type "PrimitiveComponent Object Reference") (OtherBodyIndex :type Integer) (bFromSweep :type Boolean) (SweepResult :type "HitResult Structure (by ref)"))
  (bind _returnvalue (`KismetMathLibrary.RandomFloatInRange` 1.0 6.0))
  (bind _cube (`self.Cube`))
  (bind _relativloc (`self.RelativLoc`))
  (bind _relativloc_2 (`self.RelativLoc`))
  (bind _relativloc_3 (`self.RelativLoc`))
  (cast `/Game/character/Blueprints/FirstPersonCharacter` OtherActor)
  (`|ExecutionSequence`
    (:`then_0`
      (goto _label_2 :!via `Reset`))
    (:`then_1`
      (`self.Shake`))))

(event `Shake`
  (bind _returnvalue (`KismetMathLibrary.RandomFloatInRange` 1.0 6.0))
  (bind _cube (`self.Cube`))
  (bind _relativloc (`self.RelativLoc`))
  (bind _relativloc_2 (`self.RelativLoc`))
  (bind _relativloc_3 (`self.RelativLoc`))
  (bind _counter (`/Engine/EditorBlueprintResources/StandardMacros.Do N` 6 :!label _label_2)
    (:`Exit`
      (set `self.RelativLoc` (`SceneComponent.RelativeLocation` _cube))
      (if (== _counter 5)
        (bind (_direction _newtrack_0) (`Timeline|Timeline_2` :!via `PlayFromStart`)
          (:`Update`
            (`SceneComponent.K2_SetRelativeLocation` (`self.Cube`) (`KismetMathLibrary.VLerp` _relativloc (`KismetMathLibrary.MakeVector` (.x _relativloc) (.y _relativloc) -3000.0) _newtrack_0) false false))
          (:`Finished`
            (`KismetSystemLibrary.Delay` 3.0)
            (bind (_direction_2 _newtrack_0_2) (`Timeline|Timeline_3` :!via `ReverseFromEnd`)
              (:`Update`
                (`SceneComponent.K2_SetRelativeLocation` (`self.Cube`) (`KismetMathLibrary.VLerp` _relativloc_3 (`KismetMathLibrary.MakeVector` (.x _relativloc_3) (.y _relativloc_3) -3000.0) _newtrack_0_2) false false)))))
        (else
          (bind (_direction_3 _newtrack_0_3) (`Timeline|Timeline_1` :!via `PlayFromStart`)
            (:`Update`
              (`SceneComponent.K2_SetRelativeLocation` _cube (`KismetMathLibrary.VLerp` _relativloc_2 (`KismetMathLibrary.MakeVector` (+ (.x _relativloc_2) _returnvalue) (+ (.y _relativloc_2) _returnvalue) (+ (.z _relativloc_2) _returnvalue)) _newtrack_0_3) false false))
            (:`Finished`
              (`self.Shake`))))))))

(fn `UserConstructionScript`)