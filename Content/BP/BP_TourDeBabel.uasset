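; Tower of Babel actor that rises in steps each time Grow is called and collapses once it passes its height limit.
; Grow lifts the main mesh by timeline with sound and camera shake, then increments the height held by the UI.
; Height thresholds fire escalating storm calls.
; EXPLODE resets the storm, lifts the fragment meshes, enables their physics, destroys the main mesh and pushes one piece.
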(event `self.ReceiveBeginPlay`
  (bind _componentlist (`self.componentlist`))
  (`KismetArrayLibrary.Array_Add` _componentlist (`self.StaticMesh22`))
  (`KismetArrayLibrary.Array_Add` _componentlist (`self.StaticMesh7`))
  (`KismetArrayLibrary.Array_Add` _componentlist (`self.StaticMesh15`))
  (`KismetArrayLibrary.Array_Add` _componentlist (`self.StaticMesh14`))
  (`KismetArrayLibrary.Array_Add` _componentlist (`self.StaticMesh23`))
  (`KismetArrayLibrary.Array_Add` _componentlist (`self.StaticMesh8`))
  (`KismetArrayLibrary.Array_Add` _componentlist (`self.StaticMesh16`))
  (`KismetArrayLibrary.Array_Add` _componentlist (`self.StaticMesh1`))
  (`KismetArrayLibrary.Array_Add` _componentlist (`self.StaticMesh2`))
  (`KismetArrayLibrary.Array_Add` _componentlist (`self.StaticMesh17`))
  (`KismetArrayLibrary.Array_Add` _componentlist (`self.StaticMesh9`))
  (`KismetArrayLibrary.Array_Add` _componentlist (`self.StaticMesh24`))
  (`KismetArrayLibrary.Array_Add` _componentlist (`self.StaticMesh25`))
  (`KismetArrayLibrary.Array_Add` _componentlist (`self.StaticMesh10`))
  (`KismetArrayLibrary.Array_Add` _componentlist (`self.StaticMesh18`))
  (`KismetArrayLibrary.Array_Add` _componentlist (`self.StaticMesh3`))
  (`KismetArrayLibrary.Array_Add` _componentlist (`self.StaticMesh4`))
  (`KismetArrayLibrary.Array_Add` _componentlist (`self.StaticMesh19`))
  (`KismetArrayLibrary.Array_Add` _componentlist (`self.StaticMesh11`))
  (`KismetArrayLibrary.Array_Add` _componentlist (`self.StaticMesh26`))
  (`KismetArrayLibrary.Array_Add` _componentlist (`self.StaticMesh5`))
  (`KismetArrayLibrary.Array_Add` _componentlist (`self.StaticMesh20`))
  (`KismetArrayLibrary.Array_Add` _componentlist (`self.StaticMesh12`))
  (`KismetArrayLibrary.Array_Add` _componentlist (`self.StaticMesh27`))
  (`KismetArrayLibrary.Array_Add` _componentlist (`self.StaticMesh6`))
  (`KismetArrayLibrary.Array_Add` _componentlist (`self.StaticMesh21`))
  (`KismetArrayLibrary.Array_Add` _componentlist (`self.StaticMesh13`)))

(event `Grow`
  (bind _uigeneralref (`self.UIgeneralRef`))
  (bind _newvar_0 (`self.NewVar_0`))
  (bind (_returnvalue_x _returnvalue_y _returnvalue_z) (`KismetMathLibrary.BreakVector` (`SceneComponent.K2_GetComponentLocation` (`self.StaticMesh`))))
  (bind _returnvalue (`SceneComponent.K2_GetComponentLocation` (`self.StaticMesh`)))
  (if (<= (`self.TowerHeight`) 90.75)
    (`GameplayStatics.PlaySoundAtLocation` "/Game/sound/stone-slide_Cue.stone-slide_Cue" _returnvalue (struct) 1.0 1.0 0.0 "/Game/sound/TowerAtt.TowerAtt" null null)
    (`GameplayStatics.PlayWorldCameraShake` "/Game/character/Blueprints/BabelShake.BabelShake_C" _returnvalue 10000000000.0)
    (set `self.NewVar_0` _returnvalue_z)
    (bind (_direction _newtrack_0) (`Timeline|Timeline_0` :!via `PlayFromStart`)
      (:`Update`
        (`SceneComponent.K2_SetWorldLocation` (`self.StaticMesh`) (`KismetMathLibrary.MakeVector` _returnvalue_x _returnvalue_y (`KismetMathLibrary.Lerp` _newvar_0 (+ _newvar_0 660.0) _newtrack_0)) false false))
      (:`Finished`
        (bind _output_get (set `/Game/UI/UI_general.Towerheight_UI` (+ (`/Game/UI/UI_general.Towerheight_UI` _uigeneralref) 7.0) _uigeneralref))
        (set `self.TowerHeight` _output_get)
        (`self.CheckTowerHeigh`)))
    (else
      (`self.EXPLODE`))))

(event `EXPLODE`
  (bind _staticmesh18 (`self.StaticMesh18`))
  (`self.StormNormal`)
  (for _array_element (`self.componentlist`)
    (bind (_returnvalue_x _returnvalue_y _returnvalue_z) (`KismetMathLibrary.BreakVector` (`SceneComponent.K2_GetComponentLocation` _array_element)))
    (`SceneComponent.K2_SetWorldLocation` _array_element (`KismetMathLibrary.MakeVector` _returnvalue_x _returnvalue_y (+ _returnvalue_z 8700.0)) false false))
  (`KismetSystemLibrary.Delay` 0.15)
  (for _array_element_2 (`self.componentlist`)
    (`PrimitiveComponent.SetSimulatePhysics` _array_element_2 true))
  (`ActorComponent.K2_DestroyComponent` (`self.StaticMesh`))
  (`PrimitiveComponent.AddForceAtLocation` _staticmesh18 (5000000.0 5000000.0 5000000.0) (`SceneComponent.K2_GetComponentLocation` _staticmesh18) "None"))

(fn `CheckTowerHeigh`
  (if (>= (`self.TowerHeight`) 90.0)
    (`self.StormMAX`)
    (elif (>= (`self.TowerHeight`) 72.0)
      (`self.Storm4`)
      (elif (>= (`self.TowerHeight`) 54.0)
        (`self.Storm3`)
        (elif (>= (`self.TowerHeight`) 36.0)
          (`self.Storm2`)
          (elif (>= (`self.TowerHeight`) 18.0)
            (`self.Storm1`)))))))

(fn `UserConstructionScript`)