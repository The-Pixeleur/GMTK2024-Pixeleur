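; Tutorial actor that walks the player through timed text and billboard prompts in three one-shot stages.
; ShowWelcome cycles welcome text, then calls ShowText on every BP_CAYOU actor.
; CAYOUtaken caches the player, shows congratulations text in front of the camera facing it, and reveals a billboard.
; TowerGrowth swaps billboards, then uses the cached player to place closing text likewise and steps through it before hiding it.
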(event `ShowWelcome`
  (`/Engine/EditorBlueprintResources/StandardMacros.DoOnce` false
    (:`Completed`
      (`SceneComponent.SetVisibility` (`self.TextRenderWelcome`) true false)
      (`KismetSystemLibrary.Delay` 1.5)
      (`TextRenderComponent.K2_SetText` (`self.TextRenderWelcome`) (`self.welcome2`))
      (`KismetSystemLibrary.Delay` 3.0)
      (`TextRenderComponent.K2_SetText` (`self.TextRenderWelcome`) (`self.welcome3`))
      (`KismetSystemLibrary.Delay` 3.0)
      (bind _outactors (`GameplayStatics.GetAllActorsOfClass` "/Game/BP/BP_CAYOU.BP_CAYOU_C"))
      (for _array_element _outactors
        (`/Game/BP/BP_CAYOU.ShowText` _array_element)))))

(event `CAYOUtaken`
  (bind _textrendercongrats (`self.TextRenderCongrats`))
  (bind _firstpersoncamera (`/Game/character/Blueprints/FirstPersonCharacter.FirstPersonCamera` (`self.PlayerRef`)))
  (bind _returnvalue (`SceneComponent.K2_GetComponentLocation` _firstpersoncamera))
  (`/Engine/EditorBlueprintResources/StandardMacros.DoOnce` false
    (:`Completed`
      (bind _asfirst_person_character (cast `/Game/character/Blueprints/FirstPersonCharacter` (`GameplayStatics.GetPlayerCharacter` 0)))
      (set `self.PlayerRef` _asfirst_person_character)
      (`SceneComponent.SetVisibility` (`self.TextRenderWelcome`) false false)
      (`SceneComponent.K2_SetWorldLocation` _textrendercongrats (+ (* (`KismetMathLibrary.Conv_RotatorToVector` (`SceneComponent.K2_GetComponentRotation` _firstpersoncamera)) 250.0) _returnvalue) false false)
      (`SceneComponent.K2_SetRelativeRotation` _textrendercongrats (`KismetMathLibrary.FindLookAtRotation` (`SceneComponent.K2_GetComponentLocation` (`self.TextRenderCongrats`)) _returnvalue) false false)
      (`SceneComponent.SetVisibility` (`self.TextRenderCongrats`) true false)
      (`KismetSystemLibrary.Delay` 2.5)
      (`TextRenderComponent.K2_SetText` (`self.TextRenderCongrats`) (`self.Congrats1`))
      (`SceneComponent.SetVisibility` (`self.Billboard`) true false))))

(event `TowerGrowth`
  (bind _textrenderendbasic (`self.TextRenderEndBasic`))
  (bind _textrenderendbasic_2 (`self.TextRenderEndBasic`))
  (bind _firstpersoncamera (`/Game/character/Blueprints/FirstPersonCharacter.FirstPersonCamera` (`self.PlayerRef`)))
  (bind _returnvalue (`SceneComponent.K2_GetComponentLocation` _firstpersoncamera))
  (`/Engine/EditorBlueprintResources/StandardMacros.DoOnce` false
    (:`Completed`
      (`SceneComponent.SetVisibility` (`self.Billboard`) false false)
      (`SceneComponent.SetVisibility` (`self.TextRenderCongrats`) false false)
      (`SceneComponent.SetVisibility` (`self.Billboard1`) true false)
      (`KismetSystemLibrary.Delay` 2.0)
      (`SceneComponent.SetVisibility` (`self.Billboard1`) false false)
      (`SceneComponent.SetVisibility` (`self.Billboard`) false false)
      (`SceneComponent.K2_SetWorldLocation` _textrenderendbasic (+ (* (`KismetMathLibrary.Conv_RotatorToVector` (`SceneComponent.K2_GetComponentRotation` _firstpersoncamera)) 350.0) _returnvalue) false false)
      (`SceneComponent.K2_SetRelativeRotation` _textrenderendbasic (`KismetMathLibrary.FindLookAtRotation` (`SceneComponent.K2_GetComponentLocation` (`self.TextRenderEndBasic`)) _returnvalue) false false)
      (`SceneComponent.SetVisibility` _textrenderendbasic true false)
      (`KismetSystemLibrary.Delay` 3.5)
      (`TextRenderComponent.K2_SetText` _textrenderendbasic (`self.EndBasis1`))
      (`KismetSystemLibrary.Delay` 3.0)
      (`TextRenderComponent.K2_SetText` _textrenderendbasic (`self.EndBasis2`))
      (`KismetSystemLibrary.Delay` 3.0)
      (`TextRenderComponent.K2_SetText` _textrenderendbasic_2 (`self.EndBasis3`))
      (`KismetSystemLibrary.Delay` 3.0)
      (`TextRenderComponent.K2_SetText` _textrenderendbasic_2 (`self.EndBasis5`))
      (`KismetSystemLibrary.Delay` 3.0)
      (`TextRenderComponent.K2_SetText` _textrenderendbasic_2 (`self.EndBasis6`))
      (`KismetSystemLibrary.Delay` 3.25)
      (`TextRenderComponent.K2_SetText` _textrenderendbasic_2 (`self.EndBasis7`))
      (`KismetSystemLibrary.Delay` 3.0)
      (`TextRenderComponent.K2_SetText` _textrenderendbasic_2 (`self.Endbasis8`))
      (`KismetSystemLibrary.Delay` 3.0)
      (`SceneComponent.SetVisibility` _textrenderendbasic_2 false false))))

(fn `UserConstructionScript`)